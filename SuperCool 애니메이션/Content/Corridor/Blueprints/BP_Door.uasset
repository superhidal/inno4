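; Door actor that swings open when a Character enters its trigger box and closes itself after the Character leaves.
; Overlap events set an Indoor flag, and an Opening flag blocks retriggering during the cycle.
; One timeline drives the mesh yaw open, a four-second Delay loop polls Indoor, then a second timeline plays in reverse to close.
; Opening clears after another Delay fired from the closing update.
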(event `self.Box.OnComponentBeginOverlap`
  (params (OverlappedComponent :type "PrimitiveComponent Object Reference") (OtherActor :type "Actor Object Reference") (OtherComp :type "PrimitiveComponent Object Reference") (OtherBodyIndex :type Integer) (bFromSweep :type Boolean) (SweepResult :type "HitResult Structure (by ref)"))
  (bind _sm_door (`self.SM_Door`))
  ;[1 1 1] Set indoor check near the door
  (cast `Character` OtherActor)
  (set `self.Indoor` true)
  ;[1 1 1] Check is door opening?
  (if (not (`self.Opening`))
    ;[1 1 1] Open door animation
    (set `self.Opening` true)
    (bind (_direction _door) (`Timeline|Timeline_0` :!via `PlayFromStart`)
      (:`Update`
        (`SceneComponent.K2_SetRelativeRotation` _sm_door (`KismetMathLibrary.MakeRotator` 0.0 0.0 _door) false false)
        (`KismetSystemLibrary.Delay` 4.0 :!label _label)
        ;;[1 1 1] Is the character still near the door?
        (if (`self.Indoor`)
          (goto _label)
          (else
            ;[1 1 1] Close Door Animation
            (bind (_direction_2 _door_2) (`Timeline|Timeline_1` :!via `ReverseFromEnd`)
              (:`Update`
                (`SceneComponent.K2_SetRelativeRotation` _sm_door (`KismetMathLibrary.MakeRotator` 0.0 0.0 _door_2) false false)
                (`KismetSystemLibrary.Delay` 4.0)
                (set `self.Opening` false)))))))))

(event `self.Box.OnComponentEndOverlap`
  (params (OverlappedComponent :type "PrimitiveComponent Object Reference") (OtherActor :type "Actor Object Reference") (OtherComp :type "PrimitiveComponent Object Reference") (OtherBodyIndex :type Integer))
  ;[1 1 1] Set indoor uncheck away from door
  (cast `Character` OtherActor)
  (set `self.Indoor` false))

(fn `UserConstructionScript`)