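; BP_Bullet is a weapon projectile that reacts when its StaticMesh component registers a hit.
; On hit it calls Hita on the BP_AI_Pistol found by GetActorOfClass, regardless of what was struck.
; It then stops physics and collision on Bullet, hides it, deactivates its particles and ends on a delay, without being destroyed.
; Physics impulse, player material swap and DestroyActor logic are present but disconnected.
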(event `self.ReceiveHit`
  (params (MyComp :type "PrimitiveComponent Object Reference") (Other :type "Actor Object Reference") (OtherComp :type "PrimitiveComponent Object Reference") (bSelfMoved :type Boolean) (HitLocation :type "Vector Structure") (HitNormal :type "Vector Structure") (NormalImpulse :type "Vector Structure") (Hit :type "HitResult Structure (by ref)")))

(event `self.StaticMesh.OnComponentHit`
  (params (HitComponent :type "PrimitiveComponent Object Reference") (OtherActor :type "Actor Object Reference") (OtherComp :type "PrimitiveComponent Object Reference") (NormalImpulse :type "Vector Structure") (Hit :type "HitResult Structure (by ref)"))
  (bind _bullet (`self.Bullet`))
  (bind _returnvalue (`GameplayStatics.GetActorOfClass` "/Game/AI/PistolAI/BP_AI_Pistol.BP_AI_Pistol_C"))
  (`/Game/AI/BP_AIBase.hita` _returnvalue)
  (`PrimitiveComponent.SetSimulatePhysics` _bullet false)
  (`PrimitiveComponent.SetCollisionEnabled` _bullet "NoCollision")
  (`SceneComponent.SetHiddenInGame` _bullet true false)
  (`ActorComponent.Deactivate` (`self.ParticleSystem`))
  (`KismetSystemLibrary.Delay` 4.0))

(fn `UserConstructionScript`)