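; Position is an actor Blueprint that publishes its world location and cutoff settings to the Cuotff_Collection material parameter collection.
; Its construction script writes the root's location as Position, along with the Radius, Color, Power, Boost and Hardness variables.
; The values are set only during construction, as the BeginPlay, overlap and Tick events are empty.
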(event `self.ReceiveTick`
  (params (DeltaSeconds :type "Float (single-precision)")))

(fn `UserConstructionScript`
  (`KismetMaterialLibrary.SetVectorParameterValue` "/Game/Materials/Cuotff_Collection.Cuotff_Collection" "Position" (`KismetMathLibrary.Conv_VectorToLinearColor` (`SceneComponent.K2_GetComponentLocation` (`self.DefaultSceneRoot`))))
  (`KismetMaterialLibrary.SetScalarParameterValue` "/Game/Materials/Cuotff_Collection.Cuotff_Collection" "Radius" (`self.Radius`))
  (`KismetMaterialLibrary.SetVectorParameterValue` "/Game/Materials/Cuotff_Collection.Cuotff_Collection" "Color" (`self.Color`))
  (`KismetMaterialLibrary.SetScalarParameterValue` "/Game/Materials/Cuotff_Collection.Cuotff_Collection" "Power" (`self.Power`))
  (`KismetMaterialLibrary.SetScalarParameterValue` "/Game/Materials/Cuotff_Collection.Cuotff_Collection" "Boost" (`self.Boost`))
  (`KismetMaterialLibrary.SetScalarParameterValue` "/Game/Materials/Cuotff_Collection.Cuotff_Collection" "Hardness" (`self.Hardness`)))