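; BP_NextItem is a destructible "Touch!" item that advances the game when hit.
; On BeginPlay it creates a canvas render target whose update callback draws the label and feeds the texture into a dynamic material on the Destructible via PT2D.
; A hit on the Destructible calls NextMessage on BP_StartBox, waits briefly, calls AllNextPoint on BP_Playing, then destroys the actor.
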(event `self.ReceiveBeginPlay`
  (bind _returnvalue (`CanvasRenderTarget2D.CreateCanvasRenderTarget2D` "/Script/Engine.CanvasRenderTarget2D"))
  (bind _output_get (set `self.Text` _returnvalue))
  (add `CanvasRenderTarget2D.OnCanvasRenderTargetUpdate` _output_get (delegate `DrawTextAtTexture`))
  (`CanvasRenderTarget2D.UpdateResource` _returnvalue))

(event `DrawTextAtTexture`
  (params (Canvas :type "Canvas Object Reference") (Width :type Integer) (Height :type Integer))
  (bind _destructible (`self.Destructible`))
  (`Canvas.K2_DrawText` Canvas "/Engine/EngineFonts/Roboto.Roboto" "Touch!" (-50.0 300.0) (7.0 7.0) (struct :`R` 1.0 :`G` 1.0 :`B` 1.0 :`A` 1.0) 0.0 (struct :`A` 1.0) (1.0 1.0) false false false (struct :`A` 1.0))
  (bind _returnvalue (`PrimitiveComponent.CreateDynamicMaterialInstance` _destructible 0 (`PrimitiveComponent.GetMaterial` _destructible 0) "None"))
  (`PrimitiveComponent.SetMaterial` _destructible 0 _returnvalue)
  (`MaterialInstanceDynamic.SetTextureParameterValue` _returnvalue "PT2D" (`self.Text`)))

(event `self.Destructible.OnComponentHit`
  (params (HitComponent :type "PrimitiveComponent Object Reference") (OtherActor :type "Actor Object Reference") (OtherComp :type "PrimitiveComponent Object Reference") (NormalImpulse :type "Vector Structure") (Hit :type "HitResult Structure (by ref)"))
  (bind _returnvalue (`GameplayStatics.GetActorOfClass` "/Game/Blueprints/Item/BP_StartBox.BP_StartBox_C"))
  (message `/Game/Blueprints/nextinter.next` _returnvalue)
  (`KismetSystemLibrary.PrintString` "NEXTNEXT")
  (`KismetSystemLibrary.Delay` 2.0)
  (`KismetSystemLibrary.PrintString` "delay 2sec")
  (bind _returnvalue_2 (`GameplayStatics.GetActorOfClass` "/Game/Blueprints/BP_Playing.BP_Playing_C"))
  (`/Game/Blueprints/BP_Playing.AllNextPoint` _returnvalue_2)
  (`self.K2_DestroyActor`))

(fn `UserConstructionScript`)