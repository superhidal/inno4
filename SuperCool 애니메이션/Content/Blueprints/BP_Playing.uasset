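; BP_Playing drives zone-to-zone combat progression, keyed to the AI count, and delegates spawning to the level's BP_Spawn actor.
; BeginPlay sets game-only input and spawns the player and AI for zone one.
; CheckEnemyCount triggers next-location cones at three exact AIcnt thresholds.
; AllNextPoint spawns zones two and three at the first two thresholds, while its third branch is empty.
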(event `self.ReceiveBeginPlay`
  (`WidgetBlueprintLibrary.SetInputMode_GameOnly` (`GameplayStatics.GetPlayerController` 0))
  (bind _returnvalue (`GameplayStatics.GetActorOfClass` "/Game/Blueprints/BP_Spawn.BP_Spawn_C"))
  (`/Game/Blueprints/BP_Spawn.PlayerSpawn1` _returnvalue)
  (`/Game/Blueprints/BP_Spawn.AISpawn1` _returnvalue))

(event `AllNextPoint`
  (bind _aicnt (`self.AIcnt`))
  ;[1 1 1] 장소옮겨서 플레이
  (`|ExecutionSequence`
    (:`then_0`
      (if (== _aicnt 13)
        (`KismetSystemLibrary.PrintString` "N extPoint")
        (`self.Zone2play`)))
    (:`then_1`
      (if (== _aicnt 10)
        (`self.Zone3play`)))
    (:`then_2`
      (if (== _aicnt 7)
        _))))

(event `CheckEnemyCount`
  (bind _aicnt (`self.AIcnt`))
  ;[1 1 1] 정해진 AI 수를 잡으면 장소를 옮기게 해주는 Cone이 뜨는 로직
  (`|ExecutionSequence`
    (:`then_0`
      (if (== _aicnt 13)
        (`KismetSystemLibrary.PrintString` "checknemey")
        (bind _returnvalue (`GameplayStatics.GetActorOfClass` "/Game/Blueprints/BP_Spawn.BP_Spawn_C"))
        (`/Game/Blueprints/BP_Spawn.GoNextLocation` _returnvalue)))
    (:`then_1`
      (if (== _aicnt 10)
        (bind _returnvalue_2 (`GameplayStatics.GetActorOfClass` "/Game/Blueprints/BP_Spawn.BP_Spawn_C"))
        (`/Game/Blueprints/BP_Spawn.GoNextLocation2` _returnvalue_2)))
    (:`then_2`
      (if (== _aicnt 7)
        (bind _returnvalue_3 (`GameplayStatics.GetActorOfClass` "/Game/Blueprints/BP_Spawn.BP_Spawn_C"))
        (`/Game/Blueprints/BP_Spawn.GoNextLocation3` _returnvalue_3)))))

(fn `UserConstructionScript`)

(fn `Zone2play`
  (bind _returnvalue (`GameplayStatics.GetActorOfClass` "/Game/Blueprints/BP_Spawn.BP_Spawn_C"))
  (`KismetSystemLibrary.PrintString` "zone2")
  (`/Game/Blueprints/BP_Spawn.PlayerSpawn2` _returnvalue)
  (`/Game/Blueprints/BP_Spawn.AISpawn2` _returnvalue))

(fn `Zone3play`
  (bind _returnvalue (`GameplayStatics.GetActorOfClass` "/Game/Blueprints/BP_Spawn.BP_Spawn_C"))
  (`/Game/Blueprints/BP_Spawn.PlayerSpawn3` _returnvalue)
  (`/Game/Blueprints/BP_Spawn.AISpawn3` _returnvalue))