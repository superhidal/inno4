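; Pistol-wielding enemy character that fires bullet projectiles and dies from a single damage event caused by the player.
; Construction attaches the pistol mesh to the hand socket.
; Shoot traces from the muzzle along an arrow component to aim BP_EnemyBullet, keeping the actor's yaw, and adds a muzzle flash.
; Death drops the pistol with physics, swaps the body for a destructible mesh shattered by a random impulse, then destroys the actor.
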(event `self.ReceiveTick`
  (params (DeltaSeconds :type "Float (single-precision)"))
  (`parent.ReceiveTick` DeltaSeconds))

(event `self.ReceiveAnyDamage`
  (params (Damage :type "Float (single-precision)") (DamageType :type "DamageType Object Reference") (InstigatedBy :type "Controller Object Reference") (DamageCauser :type "Actor Object Reference"))
  (bind _mesh (`self.Mesh`))
  (bind _staticmesh (`self.StaticMesh`))
  ;[1 1 1] Damage
  (cast `/Game/Blueprints/Player/BP_Player` DamageCauser)
  (if (not (`self.IsDead`))
    (set `self.IsDead` true)
    (`PrimitiveComponent.SetCollisionEnabled` (`self.CapsuleComponent`) "NoCollision")
    (`MovementComponent.StopMovementImmediately` (`self.CharacterMovement`))
    (`SceneComponent.K2_DetachFromComponent` _staticmesh "KeepWorld" "KeepWorld" "KeepWorld" true)
    (`PrimitiveComponent.SetCollisionEnabled` _staticmesh "QueryAndPhysics")
    (`PrimitiveComponent.SetSimulatePhysics` _staticmesh true)
    (`SceneComponent.SetVisibility` _mesh false false)
    (bind _returnvalue (`AddComponent|NODE_AddDestructibleComponent-0` :`RelativeTransform` (`SceneComponent.GetRelativeTransform` _mesh)))
    (`DestructibleComponent.SetDestructibleMesh` _returnvalue "/Game/Meshes/EnemyModel/EnemyModelNoRig_DM.EnemyModelNoRig_DM")
    (`PrimitiveComponent.SetSimulatePhysics` _returnvalue true)
    (`DestructibleComponent.ApplyDamage` _returnvalue 50.0 (`SceneComponent.K2_GetComponentLocation` (`self.Mesh`)) (`KismetMathLibrary.MakeVector` (`KismetMathLibrary.SelectFloat` 0.0 1.0 (`KismetMathLibrary.RandomBool`)) (`KismetMathLibrary.SelectFloat` 0.0 1.0 (`KismetMathLibrary.RandomBool`)) (`KismetMathLibrary.SelectFloat` 0.0 1.0 (`KismetMathLibrary.RandomBool`))) 500.0)
    (`KismetSystemLibrary.Delay` 1.0)
    (`self.K2_DestroyActor`)))

(event `Shoot`
  (bind (_returnvalue_roll _returnvalue_pitch _returnvalue_yaw) (`KismetMathLibrary.BreakRotator` (`self.K2_GetActorRotation`)))
  (bind _returnvalue (`SceneComponent.GetSocketLocation` (`self.StaticMesh`) "PistolMuzzle"))
  (bind (_outhit _returnvalue_2) (`KismetSystemLibrary.LineTraceSingle` _returnvalue (+ _returnvalue (* (`SceneComponent.GetForwardVector` (`self.Arrow1`)) 5000.0)) "TraceTypeQuery1"))
  (bind (_bblockinghit _binitialoverlap _time _distance _location _impactpoint _normal _impactnormal _physmat _hitactor _hitcomponent _hitbonename _hititem _faceindex _tracestart _traceend) (`GameplayStatics.BreakHitResult` _outhit))
  (`|SpawnActorFromClass` "/Game/Blueprints/Projectiles/BP_EnemyBullet.BP_EnemyBullet_C" (`KismetMathLibrary.MakeTransform` (`SceneComponent.GetSocketLocation` (`self.StaticMesh`) "PistolMuzzle") (`KismetMathLibrary.MakeRotator` (.roll (`KismetMathLibrary.FindLookAtRotation` _returnvalue (`KismetMathLibrary.SelectVector` _location _traceend _returnvalue_2))) (.pitch (`KismetMathLibrary.FindLookAtRotation` _returnvalue (`KismetMathLibrary.SelectVector` _location _traceend _returnvalue_2))) _returnvalue_yaw)) "Undefined" "OverrideRootScale" null null)
  (`GameplayStatics.SpawnEmitterAttached` "/Game/Particles/MuzzleFlash/PS_MuzzleFlash.PS_MuzzleFlash" (`self.StaticMesh`) "PistolMuzzle" (0.0 0.0 0.0) (struct) (5.0 5.0 5.0) "SnapToTarget"))

(fn `UserConstructionScript`
  (`parent.UserConstructionScript`)
  (`SceneComponent.K2_AttachToComponent` (`self.StaticMesh`) (`self.Mesh`) "PistolSocket" "SnapToTarget" "KeepRelative" "KeepRelative" true))