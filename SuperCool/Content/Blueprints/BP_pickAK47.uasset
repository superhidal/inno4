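; BP_pickAK47 is a grabbable VR AK-47 actor that motion controllers can pick up and fire.
; Pickup and Drop attach or detach it while toggling mesh physics.
; Interact flip-flops between snapping to the hand without collision and detaching with collision but physics still off, updating MotionControllerPawn's ItemRightHand for either hand.
; Action spawns a BP_Bullet at the Bullet component's world location and rotation.
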(event `/Game/VirtualRealityBP/Blueprints/PickupActorInterface.Pickup`
  (params (AttachTo :type "SceneComponent Object Reference"))
  ;[1 1 1] 코멘트
  (`PrimitiveComponent.SetSimulatePhysics` (`self.StaticMeshComponent`) false)
  (`SceneComponent.K2_AttachToComponent` (`self.K2_GetRootComponent`) AttachTo "None" "SnapToTarget" "SnapToTarget" "KeepWorld" false)
  (`SceneComponent.K2_SetRelativeLocationAndRotation` (`self.StaticMeshComponent`) (-2.0 0.0 1.0) (struct :`Yaw` -90.0) false false))

(event `/Game/VirtualRealityBP/Blueprints/PickupActorInterface.Drop`
  ;[1 1 1] 코멘트
  (`PrimitiveComponent.SetSimulatePhysics` (`self.StaticMeshComponent`) true)
  (`self.K2_DetachFromActor` "KeepWorld" "KeepWorld" "KeepWorld"))

(event `/Game/VirtualRealityBP/Blueprints/Interactable.Interact`
  (params (Hand :type "SceneComponent Object Reference"))
  (bind _staticmeshcomponent (`self.StaticMeshComponent`))
  (`/Engine/EditorBlueprintResources/StandardMacros.FlipFlop`
    (:`A`
      (`self.K2_AttachToComponent` Hand "None" "SnapToTarget" "SnapToTarget" "KeepWorld")
      (`PrimitiveComponent.SetSimulatePhysics` _staticmeshcomponent false)
      (`PrimitiveComponent.SetCollisionEnabled` _staticmeshcomponent "NoCollision")
      (`SceneComponent.K2_AddLocalRotation` _staticmeshcomponent (struct :`Yaw` -90.0) false false)
      (set `/Game/VirtualRealityBP/Blueprints/MotionControllerPawn.Item Right Hand` self (cast `/Game/VirtualRealityBP/Blueprints/MotionControllerPawn` (`GameplayStatics.GetPlayerPawn` 0) :!pure true)))
    (:`B`
      (`self.K2_DetachFromActor` "KeepWorld" "KeepWorld" "KeepWorld")
      (`PrimitiveComponent.SetSimulatePhysics` _staticmeshcomponent false)
      (`PrimitiveComponent.SetCollisionEnabled` _staticmeshcomponent "QueryAndPhysics")
      (set `/Game/VirtualRealityBP/Blueprints/MotionControllerPawn.Item Right Hand` null (cast `/Game/VirtualRealityBP/Blueprints/MotionControllerPawn` (`GameplayStatics.GetPlayerPawn` 0) :!pure true)))))

(event `/Game/VirtualRealityBP/Blueprints/Interactable.Action`
  (bind _bullet (`self.Bullet`))
  (`|SpawnActorFromClass` "/Game/Blueprints/BP_Bullet.BP_Bullet_C" (`KismetMathLibrary.MakeTransform` (`SceneComponent.K2_GetComponentLocation` _bullet) (`SceneComponent.K2_GetComponentRotation` _bullet)) "Undefined" "OverrideRootScale" null null))

(fn `UserConstructionScript`)