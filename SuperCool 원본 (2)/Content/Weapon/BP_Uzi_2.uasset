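; BP_Uzi_2 is a hand-held gun for a motion-controller pawn that can be picked up, fired and dropped.
; Interact alternates via FlipFlop between attaching to the given hand with physics and collision off, and releasing with both restored, updating the pawn's ItemRightHand.
; Action spawns a BP_Bullet at the Arrow component's transform.
; Drop detaches and re-enables physics, without restoring collision or clearing ItemRightHand.
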(event `/Game/Weapon/InteractableInterface.Interact`
  (params (Hand :type "SceneComponent Object Reference"))
  (bind _gun (`self.Gun`))
  (`/Engine/EditorBlueprintResources/StandardMacros.FlipFlop`
    (:`A`
      (`self.K2_AttachToComponent` Hand "None" "SnapToTarget" "SnapToTarget" "KeepWorld")
      (`PrimitiveComponent.SetSimulatePhysics` _gun false)
      (`PrimitiveComponent.SetCollisionEnabled` _gun "NoCollision")
      (`SceneComponent.K2_AddLocalRotation` :`self` _gun)
      (set `/Game/VirtualRealityBP/Blueprints/MotionControllerPawn.Item Right Hand` self (cast `/Game/VirtualRealityBP/Blueprints/MotionControllerPawn` (`GameplayStatics.GetPlayerPawn` 0) :!pure true)))
    (:`B`
      (`self.K2_DetachFromActor` "KeepWorld" "KeepWorld" "KeepWorld")
      (`PrimitiveComponent.SetSimulatePhysics` _gun true)
      (`PrimitiveComponent.SetCollisionEnabled` _gun "QueryAndPhysics")
      (set `/Game/VirtualRealityBP/Blueprints/MotionControllerPawn.Item Right Hand` null (cast `/Game/VirtualRealityBP/Blueprints/MotionControllerPawn` (`GameplayStatics.GetPlayerPawn` 0) :!pure true)))))

(event `/Game/Weapon/InteractableInterface.Action`
  (bind _arrow (`self.Arrow`))
  (`|SpawnActorFromClass` "/Game/Weapon/BP_Bullet.BP_Bullet_C" (`KismetMathLibrary.MakeTransform` (`SceneComponent.K2_GetComponentLocation` _arrow) (`SceneComponent.K2_GetComponentRotation` _arrow)) "Undefined" "OverrideRootScale" null null))

(event `/Game/VirtualRealityBP/Blueprints/PickupActorInterface.Drop`
  (`PrimitiveComponent.SetSimulatePhysics` (`self.Gun`) true)
  (`self.K2_DetachFromActor` "KeepWorld" "KeepWorld" "KeepWorld"))

(fn `UserConstructionScript`)