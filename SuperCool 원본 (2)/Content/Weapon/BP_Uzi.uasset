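; BP_Uzi is a gun actor that a motion controller can pick up, drop and fire.
; Pickup turns off mesh physics, snaps the actor to the controller's attach component and offsets the mesh; Drop re-enables physics and detaches it.
; Action spawns a BP_Bullet at the Arrow component's world position and rotation, with debug prints before and after.
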(event `/Game/VirtualRealityBP/Blueprints/PickupActorInterface.Pickup`
  (params (AttachTo :type "SceneComponent Object Reference"))
  (`PrimitiveComponent.SetSimulatePhysics` (`self.StaticMeshComponent`) false)
  (`SceneComponent.K2_AttachToComponent` (`self.K2_GetRootComponent`) AttachTo "None" "SnapToTarget" "SnapToTarget" "KeepWorld" false)
  (`SceneComponent.K2_SetRelativeLocationAndRotation` :`self` (`self.StaticMeshComponent`) :`NewLocation` (-4.0 0.0 -3.0)))

(event `/Game/VirtualRealityBP/Blueprints/PickupActorInterface.Drop`
  (`PrimitiveComponent.SetSimulatePhysics` (`self.StaticMeshComponent`) true)
  (`self.K2_DetachFromActor` "KeepWorld" "KeepWorld" "KeepWorld"))

(event `/Game/Weapon/InteractableInterface.Action`
  (bind _arrow (`self.Arrow`))
  (`KismetSystemLibrary.PrintString` "readyreadyreadyreadyreadyreadyready")
  (`|SpawnActorFromClass` "/Game/Weapon/BP_Bullet.BP_Bullet_C" (`KismetMathLibrary.MakeTransform` (`SceneComponent.K2_GetComponentLocation` _arrow) (`SceneComponent.K2_GetComponentRotation` _arrow)) "Undefined" "OverrideRootScale" null null)
  (`KismetSystemLibrary.PrintString` "bulletbulletbulletbulletbulletbulletbullet"))

(fn `UserConstructionScript`)